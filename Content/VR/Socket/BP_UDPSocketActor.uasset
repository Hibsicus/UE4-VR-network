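; BP_UDPSocketActor is a UDP socket actor in the VR socket folder, apparently for receiving hand data, with most logic left to its parent class.
; BeginPlay and DDataReceived only forward to the parent, while DataReceived is an empty stub.
; Tick branches on IsRightSuccess without acting on it, and a debug print of the right hand's thumb curve value is left disconnected.
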(event EventBeginPlay
  (|CallParentFunction))

(event Collision|EventActorBeginOverlap
  (params (OtherActor :type Actor%20Object%20Reference)))

(event EventTick
  (params (DeltaSeconds :type Float%20%28single-precision%29))
  (if (Variables|Default|GetisRightSuccess)
    _))

(fn ConstructionScript)

(fn DataReceived
  (return))

(fn DDataReceived
  (bind (_receivedata _sucess) (|CallParentFunction))
  (return _receivedata _sucess))